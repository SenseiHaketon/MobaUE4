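; Player character with move-to-location pathfinding, a detachable camera boom and health and mana bars.
; MoveToLocation builds a navigation path, which Tick follows point by point with movement input, using flattened 2D distance checks.
; Health and mana changes update both the controller's HUD and the overhead widget, which colors local and other players' bars differently.
; The boom detaches at start, SetCameraLocked toggles attachment, and a delayed scan sets CurrentTarget to another character.
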(event Custom|MoveToLocation
  (params (Location :type Vector))
  (if (Math|Vector|NotEqual(Vector) Location (Variables|Default|GetTargetLocation) 0.0001)
    (Variables|Default|SetTargetLocation Location)
    (bind _returnvalue (Class|NavigationSystemV1|FindPathtoLocationSynchronously (Transformation|GetActorLocation) Location self 0))
    (Variables|Default|SetTargetPath _returnvalue)
    (Variables|Default|SetCurrentPathPoint 1)))

(event Custom|UpdateManaBar
  (params (Mana :type Float%20%28single-precision%29) (MaxMana :type Float%20%28single-precision%29))
  (Utilities|FlowControl|Sequence
    (:then_0
      (bind _asbp_player_controller (Utilities|Casting|CastToBP_PlayerController (Pawn|GetController)))
      (bind _hudwidget (Variables|/Game/Blueprints/Player/BP_PlayerController.BP_PlayerController_C|GetHUDWidget _asbp_player_controller)
        (:then
          (Default|SetMana _hudwidget Mana MaxMana))
        (:else)))
    (:then_1
      (bind _aswbp_world_health_bar (Utilities|Casting|CastToWBP_WorldHealthBar (UserInterface|GetUserWidgetObject (Variables|Default|GetWorldHealthBar))))
      (Default|SetMana _aswbp_world_health_bar (/ Mana MaxMana)))))

(event Custom|UpdateHealthBar
  (params (Health :type Float%20%28single-precision%29) (MaxHealth :type Float%20%28single-precision%29))
  (Utilities|FlowControl|Sequence
    (:then_0
      (bind _asbp_player_controller (Utilities|Casting|CastToBP_PlayerController (Pawn|GetController)))
      (bind _hudwidget (Variables|/Game/Blueprints/Player/BP_PlayerController.BP_PlayerController_C|GetHUDWidget _asbp_player_controller)
        (:then
          (Default|SetHP _hudwidget Health MaxHealth))
        (:else)))
    (:then_1
      (bind _aswbp_world_health_bar (Utilities|Casting|CastToWBP_WorldHealthBar (UserInterface|GetUserWidgetObject (Variables|Default|GetWorldHealthBar))))
      (Default|SetHP _aswbp_world_health_bar Health MaxHealth))))

(event EventBeginPlay
  (|CallParentFunction)
  (Utilities|FlowControl|Sequence
    (:then_0
      (Transformation|DetachFromComponent (Variables|Default|GetCameraBoom) "KeepWorld" "KeepWorld" "KeepWorld" true)
      (Utilities|FlowControl|Delay 2.0)
      (bind _outactors (Actor|GetAllActorsOfClass "/Script/Moba.CharacterBase"))
      (for _array_element _outactors
        (if (!= _array_element self)
          (Variables|Default|SetCurrentTarget _array_element))))
    (:then_1
      (Utilities|FlowControl|Delay 0.2)
      (CallFunction|UpdateHealthBar (Class|CharacterBase|GetHealth) (Class|CharacterBase|GetMaxHealth))
      (CallFunction|UpdateManaBar (Class|CharacterBase|GetMana) (Class|CharacterBase|GetMaxMana)))
    (:then_2
      (if (Pawn|IsLocallyControlled)
        (bind _aswbp_world_health_bar (Utilities|Casting|CastToWBP_WorldHealthBar (UserInterface|GetUserWidgetObject (Variables|Default|GetWorldHealthBar))))
        (Default|SetHPBarColor _aswbp_world_health_bar "(R=0.880208,G=0.723934,B=0.000000,A=1.000000)")
        (Utilities|FlowControl|Delay 2.0)
        (bind _outactors_2 (Actor|GetAllActorsOfClass "BP_PlayerCharater_C"))
        (for _array_element_2 _outactors_2
          (if (!= _array_element_2 self)
            (bind _aswbp_world_health_bar_2 (Utilities|Casting|CastToWBP_WorldHealthBar (UserInterface|GetUserWidgetObject (Variables|BP_PlayerCharater_C|GetWorldHealthBar _array_element_2))))
            (Default|SetHPBarColor _aswbp_world_health_bar_2 "(R=0.526042,G=0.003464,B=0.000000,A=1.000000)")))))))

(event EventOnDamaged
  (params (DamageAmount :type Float%20%28single-precision%29) (HitInfo :type Hit%20Result%20Structure%20%28by%20ref%29) (DamageTags :type Gameplay%20Tag%20Container%20Structure%20%28by%20ref%29) (InstigatorCharacter :type Character%20Base%20Object%20Reference) (DamageCauser :type Actor%20Object%20Reference)))

(event EventTick
  (params (DeltaSeconds :type Float%20%28single-precision%29))
  (bind _returnvalue (Transformation|GetActorLocation))
  (bind _returnvalue_2 (Transformation|GetActorLocation))
  (bind _currentpathpoint (Variables|Default|GetCurrentPathPoint))
  (Utilities|IsValid (Variables|Default|GetTargetPath)
    (:Is%20Valid
      (Utilities|FlowControl|Sequence
        (:then_1
          (if (Utilities|Array|IsValidIndex (Variables|/Script/NavigationSystem.NavigationPath|GetPathPoints (Variables|Default|GetTargetPath)) _currentpathpoint)
            (Pawn|Input|AddMovementInput (Math|Vector|Normalize (- (Math|Vector|MakeVector (.x (Utilities|Array|Get(acopy) (Variables|/Script/NavigationSystem.NavigationPath|GetPathPoints (Variables|Default|GetTargetPath)) _currentpathpoint)) (.y (Utilities|Array|Get(acopy) (Variables|/Script/NavigationSystem.NavigationPath|GetPathPoints (Variables|Default|GetTargetPath)) _currentpathpoint)) 0.0) (Math|Vector|MakeVector (.x _returnvalue) (.y _returnvalue) 0.0))) 1.0 false)
            (if (Math|Vector|Equal(Vector) (Math|Vector|MakeVector (.x (Utilities|Array|Get(acopy) (Variables|/Script/NavigationSystem.NavigationPath|GetPathPoints (Variables|Default|GetTargetPath)) (Variables|Default|GetCurrentPathPoint))) (.y (Utilities|Array|Get(acopy) (Variables|/Script/NavigationSystem.NavigationPath|GetPathPoints (Variables|Default|GetTargetPath)) (Variables|Default|GetCurrentPathPoint))) 0.0) (Math|Vector|MakeVector (.x _returnvalue_2) (.y _returnvalue_2) 0.0) (Variables|Default|GetLocationAcceptanceRadius))
              (Math|Integer|IncrementInt (Variables|Default|GetCurrentPathPoint)))
            (else
              (Variables|Default|SetTargetPath 0))))))))

(event EventOnHealthChanged
  (params (DeltaValue :type Float%20%28single-precision%29) (EventTags :type Gameplay%20Tag%20Container%20Structure%20%28by%20ref%29))
  (CallFunction|UpdateHealthBar (Class|CharacterBase|GetHealth) (Class|CharacterBase|GetMaxHealth)))

(event EventOnManaChanged
  (params (DeltaValue :type Float%20%28single-precision%29) (EventTags :type Gameplay%20Tag%20Container%20Structure%20%28by%20ref%29))
  (CallFunction|UpdateManaBar (Class|CharacterBase|GetMana) (Class|CharacterBase|GetMaxMana)))

(fn ConstructionScript)

(fn SetCameraLocked
  (params (NewCameraLocked :type Boolean))
  (if NewCameraLocked
    (Transformation|AttachComponentToComponent (Variables|Default|GetCameraBoom) (Variables|Default|GetCapsuleComponent) "None" "SnapToTarget" "KeepWorld" "KeepWorld" true)
    (else
      (Transformation|DetachFromComponent (Variables|Default|GetCameraBoom) "KeepWorld" "KeepWorld" "KeepWorld" true))))