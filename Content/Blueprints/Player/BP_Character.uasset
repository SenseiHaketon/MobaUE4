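; BP_Character is a character Blueprint that holds champion stats and shows health on a world health bar widget.
; BeginPlay caches the WBP_WorldHealthBar from its widget component, then calls SetHealth with MaxHealth.
; SetHealth clamps CurrentHealth between zero and MaxHealth, then sets the bar to the unclamped new value divided by CurrentHealth, not MaxHealth.
; Select and Deselect events exist but are empty.
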(event EventBeginPlay
  (bind _aswbp_world_health_bar (Utilities|Casting|CastToWBP_WorldHealthBar (UserInterface|GetUserWidgetObject (Variables|Default|GetHealthBarWidget))))
  (Variables|Default|SetHealthBarWidgetBP _aswbp_world_health_bar)
  (CallFunction|SetHealth (.MaxHealth (Utilities|Struct|BreakFChampionStats (Variables|Default|GetCurrentStats)))))

(event EventSelect)

(event EventDeselect)

(fn ConstructionScript)

(fn SetHealth
  (params (NewHealth :type Integer))
  (bind _currentstats (Variables|Default|GetCurrentStats))
  (bind (_maxhealth _currenthealth) (Utilities|Struct|BreakFChampionStats _currentstats))
  (Utilities|Struct|SetmembersinFChampionStats (Variables|Default|GetCurrentStats) (Math|Integer|Clamp(Integer) NewHealth 0 _maxhealth))
  (Default|SetHealthPercent (Variables|Default|GetHealthBarWidgetBP) (/ (Math|Conversions|ToFloat(Integer) NewHealth) (Math|Conversions|ToFloat(Integer) _currenthealth))))