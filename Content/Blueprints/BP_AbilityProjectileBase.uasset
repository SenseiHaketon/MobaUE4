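; Base ability projectile that moves itself and applies a gameplay effect container spec to actors it overlaps, ignoring its instigator.
; Tick offsets it by Speed per frame without sweep or delta-time scaling, either forward or homing toward TargetActor, destroying itself if that target becomes invalid.
; Homing shots affect only their target, then destroy themselves.
; Straight shots affect each actor once and expire at MaxHitNum hits, with zero meaning unlimited.
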(event EventTick
  (params (DeltaSeconds :type Float%20%28single-precision%29))
  (if (Variables|Default|GetIsHoming)
    (bind _targetactor (Variables|Default|GetTargetActor)
      (:then
        (Transformation|AddActorWorldOffset (* (Math|Vector|Normalize (- (Transformation|GetActorLocation _targetactor) (Transformation|GetActorLocation))) (Variables|Default|GetSpeed))))
      (:else
        (Actor|DestroyActor)))
    (else
      (Transformation|AddActorWorldOffset (* (Transformation|GetActorForwardVector) (Variables|Default|GetSpeed))))))

(event Collision|EventActorBeginOverlap
  (params (OtherActor :type Actor%20Object%20Reference))
  (bind _hitactors (Variables|Default|GetHitActors))
  (if (!= OtherActor (Game|GetInstigator))
    (if (Variables|Default|GetIsHoming)
      (if (== OtherActor (Variables|Default|GetTargetActor))
        (Class|MobaBlueprintFunctionLibrary|ApplyExternalEffectContainerSpectoActors (Variables|Default|GetGameplayEffect) (Utilities|Array|MakeArray OtherActor))
        (Actor|DestroyActor))
      (elif (or (< (Utilities|Array|Length _hitactors) (Variables|Default|GetMaxHitNum)) (== (Variables|Default|GetMaxHitNum) 0))
        (if (not (Utilities|Array|ContainsItem _hitactors OtherActor))
          (Utilities|Array|Add (Variables|Default|GetHitActors) OtherActor)
          (Class|MobaBlueprintFunctionLibrary|ApplyExternalEffectContainerSpectoActors (Variables|Default|GetGameplayEffect) (Utilities|Array|MakeArray OtherActor))
          (if (and (>= (Utilities|Array|Length (Variables|Default|GetHitActors)) (Variables|Default|GetMaxHitNum)) (!= (Variables|Default|GetMaxHitNum) 0))
            (Actor|DestroyActor)))))))

(fn ConstructionScript)