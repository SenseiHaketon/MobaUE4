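; Game mode that tracks joined player controllers and rebuilds a grid visibility map from their pawn positions.
; PostLogin stores each controller, and every Tick clears and resizes the map, then converts pawn locations into grid cells scaled by map size and resolution.
; The map is a flattened square array in which only the cells occupied by player pawns are marked, with no surrounding radius.
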(event EventPostLogin
  (params (NewPlayer :type Player%20Controller%20Object%20Reference))
  (|CallParentFunction NewPlayer)
  (Utilities|Array|Add (Variables|Default|GetPlayerControllers) NewPlayer))

(event EventTick
  (params (DeltaSeconds :type Float%20%28single-precision%29))
  (Utilities|Array|Clear (Variables|Default|GetActorLocations))
  (Utilities|Array|Clear (Variables|Default|GetVisibilityMap))
  (Utilities|Array|SetArrayElem (Variables|Default|GetVisibilityMap) (- (* (Variables|Default|GetVisibilityMapResolution) (Variables|Default|GetVisibilityMapResolution)) 1) 0 true)
  (for _array_element (Variables|Default|GetPlayerControllers)
    (Utilities|Array|Add (Variables|Default|GetActorLocations) (CallFunction|WorldLocationtoGridLocation (Transformation|GetActorLocation (Pawn|GetControlledPawn _array_element)))))
  (for _array_element_2 (Variables|Default|GetActorLocations)
    (Utilities|Array|SetArrayElem (Variables|Default|GetVisibilityMap) (+ (* (Math|Float|Floor (.X (Math|Vector|BreakVector _array_element_2))) (Variables|Default|GetVisibilityMapResolution)) (Math|Float|Floor (.Y (Math|Vector|BreakVector _array_element_2)))) 1)))

(fn ConstructionScript)

(fn WorldLocationtoGridLocation
  (params (WorldLocation :type Vector))
  (bind (_x _y) (Math|Vector|BreakVector WorldLocation))
  (bind _mapsize (Variables|Default|GetMapSize))
  (bind _visibilitymapresolution (Variables|Default|GetVisibilityMapResolution))
  (return (Math|Vector|MakeVector (Math|Conversions|ToFloat(Integer) (Math|Float|Floor (* _visibilitymapresolution (/ _x (.x _mapsize))))) (Math|Conversions|ToFloat(Integer) (Math|Float|Floor (* _visibilitymapresolution (/ _y (.y _mapsize))))) 0.0)))